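; BP_mutan_enemie is a mutant enemy that chases and swipes at the paladin player.
; Seeing a BP_paladin starts AIMoveTo on player 0, with animations played directly on the mesh for running, swiping or idling.
; On arrival it box-traces along its Camera's forward vector, applies damage to a paladin hit, then repeats the chase.
; The looping attack timer's event and InfligeDegat are empty; Mort plays death but is never called here.
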(event `self.PawnSensing.OnSeePawn`
  (params (Pawn :type "Pawn Object Reference"))
  (bind _camera (`self.Camera`))
  (bind _camera_2 (`self.Camera`))
  (cast `/Game/Personnage/BP_paladin` Pawn)
  (`|AIMoveTo` self (0.0 0.0 0.0) (`GameplayStatics.GetPlayerPawn` 0) 50.0
    (:`then`
      (`SkeletalMeshComponent.PlayAnimation` (`self.Mesh`) "/Game/Personnage/animation/mutan/Goofy_Running.Goofy_Running" true))
    (:`OnSuccess`
      (`KismetSystemLibrary.K2_SetTimerDelegate` (delegate `attack`) 2.0 true)
      (`SkeletalMeshComponent.PlayAnimation` (`self.Mesh`) "/Game/Personnage/animation/mutan/Mutant_Swiping.Mutant_Swiping" false)
      (bind _outhit (`KismetSystemLibrary.BoxTraceSingleForObjects` :`Start` (+ (`SceneComponent.K2_GetComponentLocation` _camera_2) (* (`SceneComponent.GetForwardVector` _camera_2) 500)) :`End` (+ (`SceneComponent.K2_GetComponentLocation` _camera) (* (`SceneComponent.GetForwardVector` _camera) 300)) :`ObjectTypes` (`|MakeArray` "ObjectTypeQuery3" :!type "EObjectTypeQuery Enum") :`DrawDebugType` "Persistent"))
      (bind _asbp_paladin (cast `/Game/Personnage/BP_paladin` (`.HitActor` (`GameplayStatics.BreakHitResult` _outhit))))
      (`GameplayStatics.ApplyDamage` _asbp_paladin 10.0 null self))
    (:`OnFail`
      (`SkeletalMeshComponent.PlayAnimation` (`self.Mesh`) "/Game/Personnage/animation/mutan/Ninja_Idle.Ninja_Idle" true))))

(event `attack`)

(fn `inflige degat`
  (params (`point de degat` :type "Float (double-precision)")))

(fn `mort`
  (`self.DisableInput` (`GameplayStatics.GetPlayerController` 0))
  (`SkeletalMeshComponent.PlayAnimation` (`self.Mesh`) "/Game/Personnage/animation/mutan/Zombie_Death.Zombie_Death" false))

(fn `NewFunction_0`)

(fn `UserConstructionScript`)