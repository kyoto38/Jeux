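; BP_paladin is a player character Blueprint for a paladin, handling basic movement and camera input.
; Input axes drive controller yaw and pitch, and move the character relative to the control rotation's yaw only.
; Action inputs start and stop jumping and crouching, while holding sprint raises CharacterMovement's max walk speed until release.
; All logic sits in the EventGraph, and the construction script is empty.
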(event `InputAction|sprint`
  (params (Key :type "Key Structure"))
  (bind _charactermovement (`self.CharacterMovement`))
  ;[1 1 1] sprint
  (:`Pressed`
    (set `CharacterMovementComponent.MaxWalkSpeed` 600.0 _charactermovement))
  (:`Released`
    (set `CharacterMovementComponent.MaxWalkSpeed` 200.0 _charactermovement)))

(event `InputAxis|Turnn`
  (params (AxisValue :type "Float (single-precision)"))
  ;[1 1 1] camera
  (`self.AddControllerYawInput` AxisValue))

(event `InputAction|Jump`
  (params (Key :type "Key Structure"))
  ;[1 1 1] saut
  (:`Pressed`
    (`self.Jump`))
  (:`Released`
    (`self.StopJumping`)))

(event `InputAxis|LookUpp`
  (params (AxisValue :type "Float (single-precision)"))
  ;[1 1 1] camera
  (`self.AddControllerPitchInput` AxisValue))

(event `InputAxis|MoveForward`
  (params (AxisValue :type "Float (single-precision)"))
  ;[1 1 1] deplacement
  (`self.AddMovementInput` (`KismetMathLibrary.GetForwardVector` (`KismetMathLibrary.MakeRotator` 0.0 0.0 (.yaw (`self.GetControlRotation`)))) AxisValue))

(event `InputAction|crouch`
  (params (Key :type "Key Structure"))
  ;[1 1 1] crouch
  (:`Pressed`
    (`self.Crouch`))
  (:`Released`
    (`self.UnCrouch`)))

(event `InputAxis|MoveRight`
  (params (AxisValue :type "Float (single-precision)"))
  ;[1 1 1] deplacement
  (`self.AddMovementInput` (`KismetMathLibrary.GetRightVector` (`KismetMathLibrary.MakeRotator` 0.0 0.0 (.yaw (`self.GetControlRotation`)))) AxisValue))

(fn `UserConstructionScript`)