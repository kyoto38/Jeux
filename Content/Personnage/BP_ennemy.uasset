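; BP_ennemy is an enemy character that takes damage and attacks the paladin with a sword slash.
; Infligdegat lowers clamped health, playing a hit-reaction montage, or on death a single animation that disables movement and sets CounterActive, which also blocks attacks.
; attackevent plays the slash montage and immediately box-traces for pawns ahead of the camera, calling Infligdegat on any BP_paladin hit.
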(event `self.infligdegat`
  (params (pointdegat :type "Float (double-precision)"))
  (bind _vie (`self.vie`))
  (set `self.vie` (`KismetMathLibrary.FClamp` (- _vie pointdegat) 0.0 (`self.vieMax`)))
  (if (> _vie 0.0)
    (`|PlayMontage` (`self.Mesh`) "/Game/Personnage/animation/Standing_React_Large_From_Front_Montage.Standing_React_Large_From_Front_Montage" 1.5)
    (elif (not (`self.counter active`))
      (`SkeletalMeshComponent.PlayAnimation` (`self.Mesh`) "/Game/Personnage/animation/death.death" false)
      (`ActorComponent.Deactivate` (`self.CharacterMovement`))
      (set `self.counter active` true))))

(event `attackevent`
  (bind _camera (`self.Camera`))
  (bind _camera_2 (`self.Camera`))
  (if (not (`self.counter active`))
    (`|PlayMontage` (`self.Mesh`) "/Game/Personnage/animation/Stable_Sword_Outward_Slash_Montage.Stable_Sword_Outward_Slash_Montage"
      (:`then`
        (bind _outhit (`KismetSystemLibrary.BoxTraceSingleForObjects` (+ (`SceneComponent.K2_GetComponentLocation` _camera_2) (* (`SceneComponent.GetForwardVector` _camera_2) 330)) (+ (`SceneComponent.K2_GetComponentLocation` _camera) (* (`SceneComponent.GetForwardVector` _camera) 550)) (0.0 0.0 0.0) (struct) (`|MakeArray` "ObjectTypeQuery3" :!type "EObjectTypeQuery Enum")))
        (bind _asbp_paladin (cast `/Game/Personnage/BP_paladin` (`.HitActor` (`GameplayStatics.BreakHitResult` _outhit))))
        (`self.infligdegat` _asbp_paladin 20.0)))))

(fn `UserConstructionScript`
  (`parent.UserConstructionScript`))